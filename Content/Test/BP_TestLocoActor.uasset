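; Test locomotion actor for the Mover plugin that turns player run and jump input into movement commands.
; ProduceInput clamps the run axes, swaps X and Y, and rotates them by player 0's control rotation to form both move direction and orientation intent.
; These go with jump state into default character inputs, returned in a Mover input context.
; Other event and construction graphs are empty.
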(fn `ProduceInput`
  (params (SimTimeMs :type Integer))
  (returns (InputCmdResult :type "MoverInputCmdContext Structure"))
  (bind _moverdatacollection (make `MoverDataCollection`))
  (bind (_returnvalue_x _returnvalue_y) (`KismetMathLibrary.BreakVector2D` (`KismetMathLibrary.ClampAxes2D` (`|GetInputActionValue`) -1.0 1.0)))
  (bind _returnvalue (`KismetMathLibrary.GreaterGreater_VectorRotator` (`KismetMathLibrary.MakeVector` _returnvalue_y _returnvalue_x) (`Controller.GetControlRotation` (`GameplayStatics.GetPlayerController` 0))))
  (bind _characterdefaultinputs (make `CharacterDefaultInputs` _returnvalue (struct) "None" false null "None" (`|GetInputActionValue`)))
  (`MoverDataModelBlueprintLibrary.SetDirectionalInput` _characterdefaultinputs _returnvalue)
  (`MoverDataCollectionLibrary.K2_AddDataToCollection` _moverdatacollection _characterdefaultinputs)
  (return (make `MoverInputCmdContext` _moverdatacollection)))

(fn `UserConstructionScript`)