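; Test knight character driven by the Mover plugin, feeding its position to a landscape painter.
; BeginPlay caches the Landscape's location and bounds, which Tick uses to set the painter's PaintLocationUV from the actor's position.
; After a short delay it also finds and stores the CR_Couch_Knight Control Rig from the mesh's AnimInstance.
; ProduceInput builds Mover inputs from jump and control-rotated run input; predicted-trajectory debug drawing is left unconnected.
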(event `self.ReceiveTick`
  (params (DeltaSeconds :type "Float (single-precision)"))
  (bind (_returnvalue_x _returnvalue_y) (`KismetMathLibrary.BreakVector` (+ (/ (+ (`self.K2_GetActorLocation`) (`self.LandscpaeLocation`)) (`self.LandscapeSz`)) 1.0)))
  (`NiagaraComponent.SetVariableVec2` (`self.LandscapePainter`) "PaintLocationUV" (`KismetMathLibrary.MakeVector2D` _returnvalue_x _returnvalue_y)))

(event `self.ReceiveBeginPlay`
  (`|ExecutionSequence`
    (:`then_0`
      (bind _returnvalue (`GameplayStatics.GetActorOfClass` "/Script/Landscape.Landscape"))
      (set `self.LandscpaeLocation` (`self.K2_GetActorLocation` _returnvalue))
      (set `self.LandscapeSz` (* (`.BoxExtent` (`self.GetActorBounds` _returnvalue false false)) 2.0)))
    (:`then_1`
      (`KismetSystemLibrary.Delay` 0.2)
      (bind _returnvalue_2 (`ControlRig.FindControlRigs` (`SkeletalMeshComponent.GetAnimInstance` (`self.SkeletalMesh`)) "/Game/Knight/CR_Couch_Knight.CR_Couch_Knight_C"))
      (for _array_element _returnvalue_2
        (`KismetSystemLibrary.PrintString` (`KismetSystemLibrary.GetDisplayName` _array_element)))
      (bind _ascr_couch_knight (cast `/Game/Knight/CR_Couch_Knight` (`|GetArrayItem` _returnvalue_2)))
      (set `self.As CR Couch Knight` _ascr_couch_knight))))

(fn `ProduceInput`
  (params (SimTimeMs :type Integer))
  (returns (InputCmdResult :type "MoverInputCmdContext Structure"))
  (bind (_returnvalue_x _returnvalue_y) (`KismetMathLibrary.BreakVector2D` (`|GetInputActionValue`)))
  (bind _moverdatacollection (make `MoverDataCollection`))
  (bind _characterdefaultinputs (make `CharacterDefaultInputs` (0.0 0.0 90.0) (struct) "None" false null "None" (`|GetInputActionValue`)))
  (`MoverDataModelBlueprintLibrary.SetDirectionalInput` _characterdefaultinputs (`KismetMathLibrary.GreaterGreater_VectorRotator` (`KismetMathLibrary.MakeVector` _returnvalue_y _returnvalue_x) (`self.GetControlRotation`)))
  (`MoverDataCollectionLibrary.K2_AddDataToCollection` _moverdatacollection _characterdefaultinputs)
  (return (make `MoverInputCmdContext` _moverdatacollection)))

(fn `UserConstructionScript`)