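; Player knight pawn for a couch game, built on the Mover plugin with look, run and jump input.
; ProduceInput rotates the clamped run axes by control rotation and packs them with jump into Mover default inputs.
; The construction script applies a dynamic toon material to the mesh.
; EnterBreak raises an idle-break flag for five seconds, but its looping timer and the material hand-off to the anim instance are disconnected.
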(event `self.ReceiveBeginPlay`)

(event `EnterBreak`
  (set `self.inIdleBreak?` true)
  (`KismetSystemLibrary.Delay` 5.0)
  (set `self.inIdleBreak?` false))

(event `EnhancedInput|/Game/Input/Actions/IA_Look`
  (params (ActionValue :type "Vector2D Structure") (ElapsedSeconds :type "Float (double-precision)") (TriggeredSeconds :type "Float (double-precision)") (InputAction :type "InputAction Object Reference" :default "/Game/Input/Actions/IA_Look.IA_Look"))
  (:`Triggered`
    (`self.AddControllerYawInput` ActionValue_X)
    (`self.AddControllerPitchInput` (* ActionValue_Y -1.0))))

(fn `ProduceInput`
  (params (SimTimeMs :type Integer))
  (returns (InputCmdResult :type "MoverInputCmdContext Structure"))
  (bind _moverdatacollection (make `MoverDataCollection`))
  (bind (_returnvalue_x _returnvalue_y) (`KismetMathLibrary.BreakVector2D` (`KismetMathLibrary.ClampAxes2D` (`|GetInputActionValue`) -1.0 1.0)))
  (bind _returnvalue (`KismetMathLibrary.GreaterGreater_VectorRotator` (`KismetMathLibrary.MakeVector` _returnvalue_y _returnvalue_x) (`self.GetControlRotation`)))
  (bind _characterdefaultinputs (make `CharacterDefaultInputs` _returnvalue (struct) "None" false null "None" (`|GetInputActionValue`)))
  (`MoverDataModelBlueprintLibrary.SetDirectionalInput` _characterdefaultinputs _returnvalue)
  (`MoverDataCollectionLibrary.K2_AddDataToCollection` _moverdatacollection _characterdefaultinputs)
  (return (make `MoverInputCmdContext` _moverdatacollection)))

(fn `UserConstructionScript`
  (bind _returnvalue (`KismetMaterialLibrary.CreateDynamicMaterialInstance` "/Game/Knight/M_Player_Toon.M_Player_Toon"))
  (bind _output_get (set `self.KnightMat` _returnvalue))
  (`PrimitiveComponent.SetMaterial` (`self.SkeletalMesh`) 0 _output_get))